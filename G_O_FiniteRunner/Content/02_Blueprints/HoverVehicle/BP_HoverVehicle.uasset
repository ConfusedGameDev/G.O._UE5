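; BP_HoverVehicle is a player-driven hover vehicle that turns vertical and horizontal axis input into thrust and steering.
; Each Tick it counts as grounded if any of its four corner hover components is grounded, and prints that state for debugging.
; Thrust sets the MovementController's target speed only while grounded.
; Steering always sets target angular speed, multiplying the axis by its rounded value, which drops the direction sign.
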(event EventBeginPlay)

(event Collision|EventActorBeginOverlap
  (params (OtherActor :type Actor%20Object%20Reference)))

(event EventTick
  (params (DeltaSeconds :type Float%20%28single-precision%29))
  (bind _output_get (Variables|Default|SetIsGrounded (Math|Boolean|ORBoolean (Variables|/Game/02_Blueprints/HoverVehicle/HoverComponent.HoverComponent_C|GetisGrounded (Variables|Default|GetHoverComponentFL)) (Variables|/Game/02_Blueprints/HoverVehicle/HoverComponent.HoverComponent_C|GetisGrounded (Variables|Default|GetHoverComponentFR)) (Variables|/Game/02_Blueprints/HoverVehicle/HoverComponent.HoverComponent_C|GetisGrounded (Variables|Default|GetHoverComponentRL)) (Variables|/Game/02_Blueprints/HoverVehicle/HoverComponent.HoverComponent_C|GetisGrounded (Variables|Default|GetHoverComponentRR)))))
  (Development|PrintString (Utilities|String|ToString(Boolean) _output_get)))

(event Input|AxisEvents|InputAxisHorizontal
  (params (AxisValue :type Float%20%28single-precision%29))
  (Variables|/Game/02_Blueprints/HoverVehicle/BP_MovementController.BP_MovementController_C|SetTargetAngularSpeed (Variables|Default|GetMovementController) (* AxisValue (* (Variables|Default|GetSteerSpeed) (Math|Float|Round (stale Input|AxisEvents|InputAxisVertical AxisValue))))))

(event Input|AxisEvents|InputAxisVertical
  (params (AxisValue :type Float%20%28single-precision%29))
  (if (Variables|Default|GetIsGrounded)
    (Variables|/Game/02_Blueprints/HoverVehicle/BP_MovementController.BP_MovementController_C|SetTargetSpeed (Variables|Default|GetMovementController) (* AxisValue (Variables|Default|GetThrustSpeed)))))

(fn ConstructionScript)