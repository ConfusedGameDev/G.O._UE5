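; BP_LateralStabilizer is a hover vehicle component that damps the sideways sliding of its owner.
; On BeginPlay it caches the owner's root component as the physics body, provided it is a PrimitiveComponent.
; Each tick it projects linear velocity onto the body's right vector and applies an opposing force scaled by ForceFactor.
; The force is not applied as an acceleration change, so its effect depends on mass.
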(event EventBeginPlay
  (bind _asprimitive_component (Utilities|Casting|CastToPrimitiveComponent (Variables|/Script/Engine.Actor|GetRootComponent (Components|GetOwner))))
  (Variables|Default|SetBody _asprimitive_component))

(event EventTick
  (params (DeltaSeconds :type Float%20%28single-precision%29))
  (bind _body (Variables|Default|GetBody))
  (bind _body_2 (Variables|Default|GetBody)
    (:then
      (bind _returnvalue (Physics|GetPhysicsLinearVelocity _body_2 "None"))
      (Physics|AddForce _body (* (Math|Vector|GetRightVector _body) (* (Math|Vector|DotProduct _returnvalue (Math|Vector|GetRightVector _body_2)) -1.0 (Variables|Default|GetForceFactor))) "None" false))
    (:else)))