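; Movement controller for BP_HoverVehicle that drives its physics-simulated root body each tick while the vehicle is alive.
; Grounded, it applies forward force and yaw torque proportional to the gap between target and current speeds.
; Airborne, the same speed and turn targets become pitch and roll torques, with no thrust applied.
; It prints a warning when the body is not simulating physics.
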(event EventBeginPlay
  (bind _returnvalue (Components|GetOwner))
  (bind _asbp_hover_vehicle (Utilities|Casting|CastToBP_HoverVehicle _returnvalue))
  (Variables|Default|SetHoverVehicle _asbp_hover_vehicle)
  (bind _asprimitive_component (Utilities|Casting|CastToPrimitiveComponent (Variables|/Script/Engine.Actor|GetRootComponent _returnvalue)))
  (Variables|Default|SetBody _asprimitive_component))

(event EventTick
  (params (DeltaSeconds :type Float%20%28single-precision%29))
  (bind _body (Variables|Default|GetBody))
  (bind _body_2 (Variables|Default|GetBody))
  (bind _body_3 (Variables|Default|GetBody))
  (bind _body_4 (Variables|Default|GetBody))
  (bind _body_5 (Variables|Default|GetBody))
  (bind _body_6 (Variables|Default|GetBody))
  (bind _body_7 (Variables|Default|GetBody))
  (bind _body_8 (Variables|Default|GetBody)
    (:then
      (if (Physics|IsSimulatingPhysics _body_8 "None")
        (bind _hovervehicle (Variables|Default|GetHoverVehicle)
          (:then
            (if (Variables|/Game/02_Blueprints/HoverVehicle/BP_HoverVehicle.BP_HoverVehicle_C|GetisAlive _hovervehicle)
              (if (Variables|/Game/02_Blueprints/HoverVehicle/BP_HoverVehicle.BP_HoverVehicle_C|GetIsGrounded _hovervehicle)
                ;[1 1 1] Grounded Movement
                (bind _body_9 (Variables|Default|GetBody)
                  (:then
                    ;;[1 1 1] How much of the velocity is on the Forward direction
                    (bind _returnvalue (Physics|GetPhysicsLinearVelocity _body_9 "None"))
                    (Variables|Default|SetCurrentSpeed (Math|Vector|DotProduct _returnvalue (Math|Vector|GetForwardVector _body_9)))
                    ;;[1 1 1] Movement
                    (Variables|Default|SetCurrentAngularSpeed (Math|Vector|DotProduct (Physics|GetPhysicsAngularVelocityinDegrees _body "None") (Math|Vector|GetUpVector _body)))
                    (Physics|AddForce _body_4 (* (Math|Vector|GetForwardVector _body_4) (* (- (Variables|Default|GetTargetSpeed) (Variables|Default|GetCurrentSpeed)) (Variables|Default|GetSpeedToForceFactor))) "None" false)
                    ;;[1 1 1] Rotation
                    (Class|PrimitiveComponent|AddTorqueinDegrees _body_2 (* (Math|Vector|GetUpVector _body_2) (* (- (Variables|Default|GetTargetAngularSpeed) (Variables|Default|GetCurrentAngularSpeed)) (Variables|Default|GetAngularSpeedToTorqueFactor))) "None" false))
                  (:else))
                (else
                  ;[1 1 1] Air Forward Rotation
                  (Variables|Default|SetCurrentAngularAirFrontSpeed (Math|Vector|DotProduct (Physics|GetPhysicsAngularVelocityinDegrees _body_5 "None") (Math|Vector|GetRightVector _body_5)))
                  (Class|PrimitiveComponent|AddTorqueinDegrees _body_6 (* (Math|Vector|GetRightVector _body_6) (* (- (* (Variables|Default|GetTargetSpeed) (Variables|Default|Getspeed2AngularSpeed)) (Variables|Default|GetCurrentAngularAirFrontSpeed)) (Variables|Default|GetAirAngularSpeedToTorqueFactor))) "None" false)
                  ;[1 1 1] Air Forward Rotation
                  (Variables|Default|SetCurrentAngularAirLateralSpeed (Math|Vector|DotProduct (Physics|GetPhysicsAngularVelocityinDegrees _body_3 "None") (Math|Vector|GetForwardVector _body_3)))
                  (Class|PrimitiveComponent|AddTorqueinDegrees _body_7 (* (Math|Vector|GetForwardVector _body_7) (* (- (* (* (Variables|Default|GetAirLateralSpeed) (Variables|Default|GetTargetAngularSpeed)) -1.0) (Variables|Default|GetCurrentAngularAirLateralSpeed)) (Variables|Default|GetAirAngularSpeedToTorqueFactor))) "None" false)))))
          (:else))
        (else
          (Development|PrintString "no physics"))))
    (:else)))